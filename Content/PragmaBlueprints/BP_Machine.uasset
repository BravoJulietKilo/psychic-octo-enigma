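; BP_Machine is a production machine actor in the Praxis simulation, set up with test data and debug prints.
; On BeginPlay it sets the logic component's machine context, creates a test schedule and starts the component's StateTree.
; It then registers a raw-material warehouse with the inventory service and stocks it with steel bars.
; The final print shows a freshly made inventory summary, not one queried from the service.
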(event EventBeginPlay
  (bind _returnvalue (Subsystems|GetPraxisInventoryService))
  (bind _logiccomponent (Variables|Default|GetLogicComponent))
  (Variables|/Script/PraxisSimulationKernel.MachineContextComponent|SetContext (Class|MachineLogicComponent|GetMachineContextComponent _logiccomponent) (Utilities|Struct|MakePraxisMachineContext "" 1.0))
  (bind _output_get (Variables|StateTree|SetRandomService (Subsystems|GetPraxisRandomService)))
  (Class|PraxisScheduleHelpers|CreateTestSchedule 3)
  (Development|PrintString self (Utilities|String|Append "RandomService Retrieved: " (Utilities|GetDisplayName _output_get)))
  (AI|Logic|StartLogic (Class|MachineLogicComponent|GetStateTreeComponent _logiccomponent))
  (Development|PrintString self "State Tree Started")
  (Class|PraxisInventoryService|RegisterLocation _returnvalue "Warehouse_RM" "Warehouse_RM" 1e+03 100 "Zone_A")
  (Class|PraxisInventoryService|AddRawMaterial _returnvalue "Steel_Bar" 500 "Warehouse_RM" "Zone_A" 0.01)
  (bind _structout (Utilities|Struct|SetmembersinInventorySummary (Utilities|Struct|MakeInventorySummary)))
  (Development|PrintString (Utilities|String|Append (Utilities|String|ToString(Name) (.sku _structout)) (Utilities|String|ToString(Integer) (.totalquantity _structout)) "" "" (Utilities|String|ToString(Integer) (.reservedquantity _structout)) (Utilities|String|ToString(Float) (.totalvolume _structout)))))

(event Collision|EventActorBeginOverlap
  (params (OtherActor :type Actor%20Object%20Reference)))

(event EventTick
  (params (DeltaSeconds :type Float%20%28single-precision%29)))

(fn ConstructionScript)